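; BP_ProjectileBase is a projectile Blueprint that damages wizard characters it overlaps.
; On overlap, only the server acts, and only once the projectile is ready.
; A hit on any WizardCharacter other than the owning wizard deals its damage, spawns BP_ExplosionBase at its location and destroys the projectile.
; Overlaps with the owner or non-wizard actors are ignored.
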(event Collision|EventActorBeginOverlap
  (params (OtherActor :type Actor%20Object%20Reference))
  ;[1 1 1] is this the server
  (if (Ability|HasAuthority)
    ;[1 1 1] are we ready to check for collisions
    (if (Class|ProjectileBase|GetReady)
      ;[1 1 1] is this a character?
      (bind _aswizard_character (Utilities|Casting|CastToWizardCharacter OtherActor))
      ;[1 1 1] is this the character that spawned the projectile?
      (if (not (== (Class|ProjectileBase|GetWizardOwner) _aswizard_character))
        ;[1 1 1] deal damage to enemy
        (Class|WizardCharacter|TakeDamage _aswizard_character (Class|ProjectileBase|GetDamage))
        ;[1 1 1] spawn particles
        (Game|SpawnActorfromClass "/Game/Blueprints/Explosions/BP_ExplosionBase.BP_ExplosionBase_C" (Math|Transform|MakeTransform (Transformation|GetActorLocation) "0, 0, 0" "1.000000,1.000000,1.000000") "Undefined" "MultiplyWithRoot" 0 0)
        ;[1 1 1] destroy
        (Actor|DestroyActor)))))

(fn ConstructionScript)